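; BP_Light is a spotlight actor that the E key toggles on and off, with a gauge that drains while it is lit.
; ONOFFLight uses a FlipFlop to set the SpotLight's visibility and the ONLight flag.
; While ONLight is true, Tick runs a one-second Delay, then decrements Gauge and prints it on screen.
; Nothing here stops the light or the countdown when Gauge runs out.
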(event Custom|ONOFFLight
  (Utilities|FlowControl|FlipFlop
    (:A
      (Rendering|SetVisibility (Variables|Default|GetSpotLight) true false)
      (Variables|Default|SetONLight true))
    (:B
      (Rendering|SetVisibility (Variables|Default|GetSpotLight) false false)
      (Variables|Default|SetONLight false))))

(event EventBeginPlay)

(event Collision|EventActorBeginOverlap
  (params (OtherActor :type Actor%20Object%20Reference)))

(event EventTick
  (params (DeltaSeconds :type Float%20%28single-precision%29))
  (if (Variables|Default|GetONLight)
    (Utilities|FlowControl|Delay 1.0)
    (Math|Integer|DecrementInt (Variables|Default|GetGauge)
      (:%20%20
        (Development|PrintString (Utilities|String|ToString(Integer) (Variables|Default|GetGauge)) true true "(R=0.000000,G=0.660000,B=1.000000,A=1.000000)" 5.0)))))

(event Input|KeyboardEvents|E
  (params (Key :type Key%20Structure :default "None"))
  (:Pressed
    (CallFunction|ONOFFLight)))

(fn ConstructionScript)